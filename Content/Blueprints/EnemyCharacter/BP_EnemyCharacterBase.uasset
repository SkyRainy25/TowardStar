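; Base enemy character Blueprint that handles the visual entrance and death of enemies.
; On BeginPlay, a reversed timeline undissolves the mesh and equipped weapon while a random entry montage plays.
; On death, it freezes animation, disables capsule collision, removes UI widgets, dissolves both meshes and async-loads a Niagara effect tinted to the dissolve edge color.
; When dissolved, it destroys the weapon, activates the item-spawn ability and destroys itself after a delay.
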(event `self.ReceiveBeginPlay`
  (bind _entry_montages_to_play (`self.Entry Montages To Play`))
  (bind _returnvalue (`PawnCombatComponent.GetCharacterCurrentEquippedWeapon` (`self.EnemyCombatComponent`)))
  (`|ExecutionSequence`
    (:`then_0`
      (`TimelineComponent.SetPlayRate` (`self.Entry RestoreTimeLine`) (/ 1.0 (`self.Total Entry Restore Time`)))
      (bind (_direction _dissolve) (`Timeline|Entry RestoreTimeLine` :!via `ReverseFromEnd`)
        (:`Update`
          (`MeshComponent.SetScalarParameterValueOnMaterials` (`self.Mesh`) "DissolveAmount" _dissolve)
          (`/Engine/EditorBlueprintResources/StandardMacros.IsValid` _returnvalue
            (:`Is Valid`
              (`MeshComponent.SetScalarParameterValueOnMaterials` (`StarWeaponBase.StaticWeaponMesh` _returnvalue) "DissolveAmount" _dissolve))))))
    (:`then_1`
      (if (`KismetArrayLibrary.Array_IsNotEmpty` _entry_montages_to_play)
        (`self.PlayAnimMontage` (`KismetArrayLibrary.Array_Random` _entry_montages_to_play))))))

(event `/Game/Blueprints/EnemyCharacter/BPI_EnemyDeath.OnEnemyDied`
  (params (DissolveNiagaraSystem :type "NiagaraSystem Soft Object Reference"))
  (bind _mesh (`self.Mesh`))
  (bind _returnvalue (`PawnCombatComponent.GetCharacterCurrentEquippedWeapon` (`self.EnemyCombatComponent`)))
  (`|ExecutionSequence`
    (:`then_0`
      ;[1 1 1] Stop Playing Anim
      (set `SkeletalMeshComponent.bPauseAnims` true (`self.Mesh`))
      ;[1 1 1] Set No Collision to CapsuleComp
      (`PrimitiveComponent.SetCollisionEnabled` (`self.CapsuleComponent`) "NoCollision"))
    (:`then_1`
      (`TimelineComponent.SetPlayRate` (`self.DissolveTimeLine`) (/ 1.0 (`self.TotalDissolveTime`)))
      (bind (_direction _dissolve) (`Timeline|DissolveTimeLine` :!via `PlayFromStart`)
        (:`Update`
          ;[1 1 1] Apply Dissolve Effect to Enemy
          (`MeshComponent.SetScalarParameterValueOnMaterials` (`self.Mesh`) "DissolveAmount" _dissolve)
          (`/Engine/EditorBlueprintResources/StandardMacros.IsValid` _returnvalue
            (:`Is Valid`
              ;[1 1 1] Apply Dissolve FX to Weapon
              (`MeshComponent.SetScalarParameterValueOnMaterials` (`StarWeaponBase.StaticWeaponMesh` _returnvalue) "DissolveAmount" _dissolve))))
        (:`Finished`
          (`self.DastroyEnemyAndWeapon`)
          (`KismetSystemLibrary.Delay` 0.5)
          (`self.K2_DestroyActor`))))
    (:`then_2`
      ;[1 1 1] Remove HealthBar
      (`EnemyUIComponent.RemoveEnemyDrawnWidgetsIfAny` (`self.EnemyUIComponent`)))
    (:`then_3`
      (bind _object (`|LoadAsset` DissolveNiagaraSystem)
        (:`Completed`
          (bind `_as나이아가라_시스템` (cast `NiagaraSystem` _object))
          (bind _returnvalue_2 (`NiagaraFunctionLibrary.SpawnSystemAttached` `_as나이아가라_시스템` (`self.Mesh`) "None" (0.0 0.0 0.0) (struct) "KeepRelativeOffset" true))
          ;[1 1 1] Match NaigaraSystem Effect Color with Dissolve Effect
          (bind _returnvalue_3 (`PrimitiveComponent.CreateDynamicMaterialInstance` _mesh 0 (`PrimitiveComponent.GetMaterial` _mesh 0) "None"))
          (bind _returnvalue_4 (`MaterialInstanceDynamic.K2_GetVectorParameterValue` _returnvalue_3 "DissolveEdgeColor"))
          (`NiagaraComponent.SetNiagaraVariableLinearColor` _returnvalue_2 "DissolveParticleColor" _returnvalue_4))))))

(fn `DastroyEnemyAndWeapon`
  (bind _returnvalue (`PawnCombatComponent.GetCharacterCurrentEquippedWeapon` (`self.EnemyCombatComponent`)))
  (`/Engine/EditorBlueprintResources/StandardMacros.IsValid` _returnvalue
    (:`Is Valid`
      (`self.K2_DestroyActor` _returnvalue))
    (:`Is Not Valid`
      _))
  (`StarAbilitySystemComponent.TryActivateAbilityByTag` (`self.StarAbilitySystemComponent`) (struct :`TagName` "Enemy.Ability.SpawnItem")))

(fn `UserConstructionScript`)