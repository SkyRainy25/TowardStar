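; BP_Boss is the boss enemy character, using Frost Giant animation, that reacts to tornado projectiles and energy balls.
; On BeginPlay it plays the intro montage, saves its spawn location to the Blackboard and deactivates its Niagara effect.
; A Sphere overlap calls DestroyShield for a tornado projectile, or prints a debug string and calls EnergyBallOverlapped for an energy ball.
; Tick is disabled, and the capsule overlap event is empty.
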(event `self.ReceiveActorBeginOverlap`
  (params (OtherActor :type "Actor Object Reference"))
  (`parent.ReceiveActorBeginOverlap` OtherActor))

(event `self.ReceiveBeginPlay`
  (`parent.ReceiveBeginPlay`)
  (`self.PlayAnimMontage` "/Game/Blueprints/EnemyCharacter/FrostGiant/Montage/AM_FrostGiant_Intro.AM_FrostGiant_Intro")
  (`BlackboardComponent.SetValueAsVector` (`AIBlueprintHelperLibrary.GetBlackboard` null) "SpawnLocation" (`self.K2_GetActorLocation`))
  (`ActorComponent.Deactivate` (`self.Niagara`)))

(event `self.Sphere.OnComponentBeginOverlap`
  (params (OverlappedComponent :type "PrimitiveComponent Object Reference") (OtherActor :type "Actor Object Reference") (OtherComp :type "PrimitiveComponent Object Reference") (OtherBodyIndex :type Integer) (bFromSweep :type Boolean) (SweepResult :type "HitResult Structure (by ref)"))
  (cast `/Game/Blueprints/PlayerCharacter/BP_Projectile_Tornado` OtherActor
    (:`then`
      (`self.DestroyShield`))
    (:`CastFailed`
      (cast `/Game/Blueprints/EnemyCharacter/Boss/BP_EnergyBall` OtherActor)
      (`KismetSystemLibrary.PrintString` "Hello")
      (`self.EnergyBallOverlapped`))))

(event `self.CapsuleComponent.OnComponentBeginOverlap`
  (params (OverlappedComponent :type "PrimitiveComponent Object Reference") (OtherActor :type "Actor Object Reference") (OtherComp :type "PrimitiveComponent Object Reference") (OtherBodyIndex :type Integer) (bFromSweep :type Boolean) (SweepResult :type "HitResult Structure (by ref)")))

(fn `UserConstructionScript`
  (`parent.UserConstructionScript`))