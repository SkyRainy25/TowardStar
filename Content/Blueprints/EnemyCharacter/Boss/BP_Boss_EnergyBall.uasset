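; BP_Boss_EnergyBall is the boss's energy ball projectile, handling impact feedback when it hits.
; The OnSpawnProjectileHitFX event plays the impact sound and spawns the impact Niagara effect at the hit location, each only if its asset is valid.
; The overlap event casts to BP_Boss but does nothing further.
; Movement deactivation and actor destruction nodes are left unconnected, so they never run here.
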(event `self.ReceiveBeginPlay`)

(event `self.ReceiveActorBeginOverlap`
  (params (OtherActor :type "Actor Object Reference"))
  (cast `/Game/Blueprints/EnemyCharacter/Boss/BP_Boss` OtherActor))

(event `self.BP_OnSpawnProjectileHitFX`
  (params (HitLocation :type "Vector Structure (by ref)"))
  (set `self.Hit Location` HitLocation)
  (`|ExecutionSequence`
    (:`then_0`
      (bind _projectile_impact_sound (`self.Projectile Impact Sound`)
        (:`then`
          (`GameplayStatics.PlaySoundAtLocation` _projectile_impact_sound (`self.Hit Location`) (struct) 1.0 1.0 0.0 null null null null))
        (:`else`)))
    (:`then_1`
      (bind _projectile_impact_fx (`self.Projectile Impact FX`)
        (:`then`
          (`NiagaraFunctionLibrary.SpawnSystemAtLocation` _projectile_impact_fx (`self.Hit Location`)))
        (:`else`)))))

(fn `UserConstructionScript`)