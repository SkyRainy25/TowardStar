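; Boss-folder test obstacle that hero weapons can break and that expires on its own after about six seconds.
; Each BP_HeroWeaponBase overlap lowers DurationNum, playing a small hit sound at world origin until the count runs out.
; Tick accumulates the lifetime, and both depletion and the Destroyed event share the fire explosion, sound and destroy path.
; BeginPlay starts a timeline with no visible update logic.
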(event `self.ReceiveBeginPlay`
  (`Timeline|타임라인`))

(event `self.ReceiveActorBeginOverlap`
  (params (OtherActor :type "Actor Object Reference"))
  (bind _returnvalue (`self.K2_GetActorLocation`))
  (cast `/Game/Blueprints/PlayerCharacter/HeroWeapons/BP_HeroWeaponBase` OtherActor)
  (bind _result (`/Engine/EditorBlueprintResources/StandardMacros.DecrementInt` (`self.DurationNum`))
    (:`  `
      (if (<= _result 0)
        (`GameplayStatics.PlaySoundAtLocation` "/Game/AuraAssets/Sounds/Abilities/FireBolt/wav/Impact/SFX_Fireball_Hit_03.SFX_Fireball_Hit_03" _returnvalue (struct) 1.0 1.0 0.0 null null null null :!label _label)
        (`NiagaraFunctionLibrary.SpawnSystemAtLocation` "/Game/AuraAssets/Effects/Projectiles/FireExplosion/NS_FireExplosion.NS_FireExplosion" _returnvalue)
        (`self.K2_DestroyActor`)
        (else
          (`GameplayStatics.PlaySoundAtLocation` "/Game/AuraAssets/Sounds/Abilities/FireBolt/wav/Impact/SFX_SmallFireball_Hit_03.SFX_SmallFireball_Hit_03" (0.0 0.0 0.0) (struct) 1.0 1.0 0.0 null null null null))))))

(event `self.ReceiveDestroyed`
  (goto _label))

(event `self.ReceiveTick`
  (params (DeltaSeconds :type "Float (single-precision)"))
  (bind _output_get (set `self.DurationTime` (+ DeltaSeconds (`self.DurationTime`))))
  (if (>= _output_get 6.0)
    (`self.K2_DestroyActor`)))

(fn `UserConstructionScript`)