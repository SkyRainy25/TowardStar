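; Base game mode that triggers the win screen once every enemy in the level is gone.
; On BeginPlay it gathers all BP_EnemyCharacterBase actors, then prunes invalid entries every Tick, so enemies spawned later are not tracked.
; When the list empties, a one-shot flag starts a delayed sequence that clears widgets, fades the camera out, then async-loads and displays WBP_WinScreen.
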(event `self.ReceiveBeginPlay`
  (bind _outactors (`GameplayStatics.GetAllActorsOfClass` "/Game/Blueprints/EnemyCharacter/BP_EnemyCharacterBase.BP_EnemyCharacterBase_C"))
  (set `self.Out Actors` _outactors)
  (set `self.HasEnded` false))

(event `self.ReceiveTick`
  (params (DeltaSeconds :type "Float (single-precision)"))
  (for _array_element (`self.Out Actors`)
    (`/Engine/EditorBlueprintResources/StandardMacros.IsValid` _array_element
      (:`Is Not Valid`
        (`KismetArrayLibrary.Array_RemoveItem` (`self.Out Actors`) _array_element))))
  (if (`self.HasEnded`)
    _
    (elif (== (`KismetArrayLibrary.Array_Length` (`self.Out Actors`)) 0)
      (set `self.HasEnded` true)
      (`KismetSystemLibrary.Delay` 2.0)
      (`WidgetLayoutLibrary.RemoveAllWidgets`)
      (`PlayerCameraManager.StartCameraFade` :`self` (`GameplayStatics.GetPlayerCameraManager` 0) :`ToAlpha` 1.0 :`Duration` 3.0 :`bHoldWhenFinished` true)
      (`KismetSystemLibrary.Delay` 3.0)
      (bind _class (`|LoadAssetClass` "/Game/Blueprints/Widgets/GameModeWidgets/WBP_WinScreen.WBP_WinScreen_C")
        (:`Completed`
          (bind `_as사용자_위젯` (castclass `UserWidget` _class))
          (bind _returnvalue (`|CreateWidget` `_as사용자_위젯`))
          (`UserWidget.AddToViewport` _returnvalue 0))))))

(fn `UserConstructionScript`)