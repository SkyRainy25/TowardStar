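; Gameplay cue that shows an unblockable-attack warning effect on an enemy when executed.
; It spawns the Niagara warning system at the target's eye viewpoint, pushed along the actor's forward vector and facing that direction.
; The cue's raw magnitude sets the forward offset distance.
; The spawned effect is then attached to the target's root component with KeepRelative rules before the parent OnExecute runs.
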(fn `OnExecute`
  (params (MyTarget :type "Actor Object Reference") (Parameters :type "GameplayCueParameters Structure (by ref)"))
  (returns (ReturnValue :type Boolean))
  ;[1 1 1] Spawn Warning FX
  (bind _returnvalue (`NiagaraFunctionLibrary.SpawnSystemAtLocation` null "/Game/Assets/Niagara/Warning/NS_UnbloackableWarning.NS_UnbloackableWarning" (+ (`Actor.GetActorEyesViewPoint` (`local.MyTarget`)) (* (`Actor.GetActorForwardVector` (`local.MyTarget`)) (`.RawMagnitude` (`AbilitySystemBlueprintLibrary.BreakGameplayCueParameters` (`local.Parameters`))))) (`KismetMathLibrary.Conv_VectorToRotator` (`Actor.GetActorForwardVector` (`local.MyTarget`)))))
  ;[1 1 1] Attach
  (`SceneComponent.K2_AttachToComponent` _returnvalue (`Actor.RootComponent` (`local.MyTarget`)) "None" "KeepRelative" "KeepRelative" "KeepRelative" true)
  (return (`parent.OnExecute` (`local.MyTarget`) (`local.Parameters`))))