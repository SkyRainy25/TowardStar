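; BP_StarHeroCharacter2 is a player character Blueprint that handles pause menu and Fire Tornado input through Enhanced Input.
; The pause action async-loads the WBP_PauseScreen class on demand, then creates the widget and adds it to the viewport.
; Holding Fire Tornado for two seconds marks the charge complete; that state and elapsed time go to CallInputButtonReleased.
; Cancelling or completing the input clears the charge flag before making the same call.
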(event `self.ReceiveBeginPlay`)

(event `EnhancedInput|/Game/Blueprints/Input/Actions/IA_PauseMenu`
  (params (ActionValue :type Boolean) (ElapsedSeconds :type "Float (double-precision)") (TriggeredSeconds :type "Float (double-precision)") (InputAction :type "InputAction Object Reference" :default "/Game/Blueprints/Input/Actions/IA_PauseMenu.IA_PauseMenu"))
  (:`Started`
    (bind _class (`|LoadAssetClass` "/Game/Blueprints/Widgets/GameModeWidgets/WBP_PauseScreen.WBP_PauseScreen_C")
      (:`Completed`
        (bind `_as사용자_위젯` (castclass `UserWidget` _class))
        (bind _returnvalue (`|CreateWidget` `_as사용자_위젯`))
        (`UserWidget.AddToViewport` _returnvalue 0)))))

(event `EnhancedInput|/Game/Blueprints/Input/Actions/IA_FireTornado`
  (params (ActionValue :type Boolean) (ElapsedSeconds :type "Float (double-precision)") (TriggeredSeconds :type "Float (double-precision)") (InputAction :type "InputAction Object Reference" :default "/Game/Blueprints/Input/Actions/IA_FireTornado.IA_FireTornado"))
  (:`Triggered`
    (if (>= ElapsedSeconds 2.0)
      (set `self.bIsChargingCompleted` true)
      (`self.InputButtonReleased` ElapsedSeconds (`self.bIsChargingCompleted`) :!label _label)))
  (:`Canceled`
    (set `self.bIsChargingCompleted` false :!label _label_2)
    (goto _label))
  (:`Completed`
    (goto _label_2)))

(fn `UserConstructionScript`)