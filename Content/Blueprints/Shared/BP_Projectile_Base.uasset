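; Base projectile Blueprint that handles the sound and visual effects for a projectile's spawn, flight and impact.
; BeginPlay plays a spawn sound, attaches a flying sound to the root and spawns a Niagara muzzle effect, rotated from the actor's location vector.
; OnSpawnProjectileHitFX plays the impact sound and effect at a supplied hit location.
; Each asset is validity-checked, so any can be left unset; movement and hit detection are not in these graphs.
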(event `self.BP_OnSpawnProjectileHitFX`
  (params (HitLocation :type "Vector Structure (by ref)"))
  (set `self.Hit Location` HitLocation)
  (`|ExecutionSequence`
    (:`then_0`
      (bind _projectileimpactsound (`self.ProjectileImpactSound`)
        (:`then`
          (`GameplayStatics.PlaySoundAtLocation` _projectileimpactsound (`self.Hit Location`) (struct) 1.0 1.0 0.0 null null null null))
        (:`else`)))
    (:`then_1`
      (bind _projectileimpactfx (`self.ProjectileImpactFX`)
        (:`then`
          (`NiagaraFunctionLibrary.SpawnSystemAtLocation` _projectileimpactfx (`self.Hit Location`)))
        (:`else`)))))

(event `self.ReceiveBeginPlay`
  (bind _returnvalue (`self.K2_GetActorLocation`))
  (`|ExecutionSequence`
    (:`then_0`
      (bind _projectilespawnsound (`self.ProjectileSpawnSound`)
        (:`then`
          (`GameplayStatics.PlaySoundAtLocation` _projectilespawnsound (`self.K2_GetActorLocation`) (struct) 1.0 1.0 0.0 null null null null))
        (:`else`)))
    (:`then_1`
      (bind _projectileflyingsound (`self.ProjectileFlyingSound`)
        (:`then`
          (`GameplayStatics.SpawnSoundAttached` _projectileflyingsound (`self.RootComponent`) "None" (0.0 0.0 0.0) (struct) "KeepRelativeOffset" true 1.0 1.0 0.0 null null))
        (:`else`)))
    (:`then_2`
      (bind _projectilemuzzleeffect (`self.ProjectileMuzzleEffect`)
        (:`then`
          (`NiagaraFunctionLibrary.SpawnSystemAtLocation` _projectilemuzzleeffect _returnvalue (`KismetMathLibrary.Conv_VectorToRotator` _returnvalue)))
        (:`else`)))))

(fn `UserConstructionScript`)